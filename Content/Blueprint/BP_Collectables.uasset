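; BP_Collectables is a collectable actor that the player picks up with the Interaction input.
; Its Box overlap with BP_PlayerBase toggles input on the actor and shows or removes the WBP_Interact prompt.
; Pressing Interaction decrements CollactablesLeft on BP_GameModeBase, adds a WBP_Collectables widget to the viewport and destroys the actor.
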(event OnComponentBeginOverlap(Box)
  (params (OverlappedComponent :type Primitive%20Component%20Object%20Reference) (OtherActor :type Actor%20Object%20Reference) (OtherComp :type Primitive%20Component%20Object%20Reference) (OtherBodyIndex :type Integer) (bFromSweep :type Boolean) (SweepResult :type Hit%20Result%20Structure%20%28by%20ref%29))
  (Utilities|Casting|CastToBP_PlayerBase OtherActor)
  (Input|EnableInput (Game|GetPlayerController 0))
  (bind _returnvalue (UserInterface|CreateWidget "/Game/Blueprint/Widgets/WBP_Interact.WBP_Interact_C"))
  (UserInterface|Viewport|AddtoViewport _returnvalue 0))

(event OnComponentEndOverlap(Box)
  (params (OverlappedComponent :type Primitive%20Component%20Object%20Reference) (OtherActor :type Actor%20Object%20Reference) (OtherComp :type Primitive%20Component%20Object%20Reference) (OtherBodyIndex :type Integer))
  (Utilities|Casting|CastToBP_PlayerBase OtherActor)
  (Input|DisableInput (Game|GetPlayerController 0))
  (bind _foundwidgets (Widget|GetAllWidgetsOfClass "/Game/Blueprint/Widgets/WBP_Interact.WBP_Interact_C" true))
  (Widget|RemovefromParent _foundwidgets))

(event Input|ActionEvents|InputActionInteraction
  (params (Key :type Key%20Structure :default "None"))
  (:Pressed
    (bind _asbp_game_mode_base (Utilities|Casting|CastToBP_GameModeBase (Game|GetGameMode)))
    (bind _result (Math|Integer|DecrementInt (Variables|/Game/Blueprint/BP_GameModeBase.BP_GameModeBase_C|GetCollactablesLeft _asbp_game_mode_base))
      (:%20%20
        (Variables|/Game/Blueprint/BP_GameModeBase.BP_GameModeBase_C|SetCollactablesLeft _asbp_game_mode_base _result)
        (bind _returnvalue (UserInterface|CreateWidget "/Game/Blueprint/Widgets/WBP_Collectables.WBP_Collectables_C"))
        (UserInterface|Viewport|AddtoViewport _returnvalue 0)
        (Actor|DestroyActor)))))

(fn ConstructionScript)